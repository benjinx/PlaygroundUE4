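; Player controller Blueprint that provides click-to-move for the controlled pawn.
; MoveToHitLocation takes a hit result, prints a debug string and calls SimpleMoveToLocation toward the hit point, skipping points closer to the pawn than MinClickDistance.
; The event graph and construction script are empty, and nothing in this Blueprint calls the function.
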(fn `MoveToHitLocation`
  (params (Hit :type "HitResult Structure"))
  (bind (_bblockinghit _binitialoverlap _time _distance _location) (`GameplayStatics.BreakHitResult` Hit))
  (`KismetSystemLibrary.PrintString` "Hit")
  (if (>= (`KismetMathLibrary.VSize` (- (`self.K2_GetActorLocation` (`self.K2_GetPawn`)) _location)) (`self.MinClickDistance`))
    (`AIBlueprintHelperLibrary.SimpleMoveToLocation` self _location)))

(fn `UserConstructionScript`)